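; BP_TelekineticProp is a telekinesis prop actor that exposes visual-effect hooks, with no movement or physics logic in its graphs.
; Events activate and deactivate its Niagara component, set its spawn rate and pass it the actor's location through user parameters.
; ActivateTrails sets only the spawn rate, without activating the system.
; SpawnSparks spawns a separate one-shot NS_Sparks system at the actor, oriented by the normalized impulse through a Direction parameter.
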(event EventActivateParticleSystem
  (bind _niagara (Variables|Default|GetNiagara))
  (Components|Activation|Activate _niagara false)
  (Audio|Parameter|SetFloatParameter _niagara "Spawn0" (Variables|Default|GetNiagaraSpawnRate) :!class /Script/AudioExtensions.AudioParameterControllerInterface))

(event EventFeedLocationtoParticleSystem
  (Effects|Components|ParticleSystem|SetVectorParameter (Variables|Default|GetNiagara) "Location0" (Transformation|GetActorLocation)))

(event EventDeactivateParticleSystem
  (Components|Activation|Deactivate (Variables|Default|GetNiagara)))

(event EventSpawnSparks
  (params (Impulse :type Vector%20%28by%20ref%29 :default "0, 0, 0"))
  (bind _returnvalue (Niagara|SpawnSystematLocation "/Game/VFX/NS_Sparks.NS_Sparks" (Transformation|GetActorLocation)))
  (Effects|Components|ParticleSystem|SetVectorParameter _returnvalue "Direction" (Math|Vector|Normalize Impulse)))

(fn ConstructionScript)

(fn ActivateTrails
  (Audio|Parameter|SetFloatParameter (Variables|Default|GetNiagara) "Spawn0" (Variables|Default|GetNiagaraSpawnRate) :!class /Script/AudioExtensions.AudioParameterControllerInterface))